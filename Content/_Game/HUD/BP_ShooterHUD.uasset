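; HUD class that draws a dynamic four-piece crosshair for the shooter character.
; On BeginPlay it caches the player pawn as BP_ShooterCharacter.
; Each DrawHUD call finds the screen center and draws top, bottom, left and right crosshair textures, pushed outward by the character's crosshair spread multiplier scaled by a maximum spread.
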(event `self.ReceiveBeginPlay`
  ;[1 1 1] получение ссылки
  (`/Engine/EditorBlueprintResources/StandardMacros.IsValid` (`self.ShooterCharacter`)
    (:`Is Not Valid`
      (bind _asbp_shooter_character (cast `/Game/_Game/Character/Blueprint/BP_ShooterCharacter` (`GameplayStatics.GetPlayerPawn` 0)))
      (set `self.ShooterCharacter` _asbp_shooter_character))))

(event `self.ReceiveDrawHUD`
  (params (SizeX :type Integer) (SizeY :type Integer))
  (bind (_crosshairbasecenter_x _crosshairbasecenter_y) (`KismetMathLibrary.BreakVector2D` (`self.CrosshairBaseCenter`)))
  (bind (_crosshairbasecenter_x_2 _crosshairbasecenter_y_2) (`KismetMathLibrary.BreakVector2D` (`self.CrosshairBaseCenter`)))
  (bind (_crosshairbasecenter_x_3 _crosshairbasecenter_y_3) (`KismetMathLibrary.BreakVector2D` (`self.CrosshairBaseCenter`)))
  (bind (_crosshairbasecenter_x_4 _crosshairbasecenter_y_4) (`KismetMathLibrary.BreakVector2D` (`self.CrosshairBaseCenter`)))
  (bind (_x _y) (`KismetMathLibrary.BreakVector2D` (`self.ScreenCenter`)))
  (set `self.ScreenCenter` (`KismetMathLibrary.MakeVector2D` (`KismetMathLibrary.Conv_IntToDouble` (/ SizeX 2)) (`KismetMathLibrary.Conv_IntToDouble` (/ SizeY 2))))
  ;[1 1 1] получение умножителя перекрестия
  (set `self.CrosshairSpreadMultiplier` (`ShooterCharacter.GetCrosshairSpreadMultiplier` (`self.ShooterCharacter`)))
  ;[1 1 1] центр перекрестия
  (set `self.CrosshairBaseCenter` (`KismetMathLibrary.MakeVector2D` (- _x (`self.CrosshairHalfWidth`)) (- _y (`self.CrosshairHalfHeight`))))
  (`self.DrawTexture` "/Game/_Game/Assets/Texture/Crosshairs/Crosshair_Quad_9_Bottom.Crosshair_Quad_9_Bottom" _crosshairbasecenter_x (+ _crosshairbasecenter_y (* (`self.CrosshairSpreadMultiplier`) (`self.CrosshairSpreadMax`))) 64.0 64.0 0.0 0.0 1.0 1.0)
  (`self.DrawTexture` "/Game/_Game/Assets/Texture/Crosshairs/Crosshair_Quad_9_Top.Crosshair_Quad_9_Top" _crosshairbasecenter_x_2 (- _crosshairbasecenter_y_2 (* (`self.CrosshairSpreadMultiplier`) (`self.CrosshairSpreadMax`))) 64.0 64.0 0.0 0.0 1.0 1.0)
  (`self.DrawTexture` "/Game/_Game/Assets/Texture/Crosshairs/Crosshair_Quad_9_Right.Crosshair_Quad_9_Right" (+ _crosshairbasecenter_x_4 (* (`self.CrosshairSpreadMultiplier`) (`self.CrosshairSpreadMax`))) _crosshairbasecenter_y_4 64.0 64.0 0.0 0.0 1.0 1.0)
  (`self.DrawTexture` "/Game/_Game/Assets/Texture/Crosshairs/Crosshair_Quad_9_Left.Crosshair_Quad_9_Left" (- _crosshairbasecenter_x_3 (* (`self.CrosshairSpreadMultiplier`) (`self.CrosshairSpreadMax`))) _crosshairbasecenter_y_3 64.0 64.0 0.0 0.0 1.0 1.0))

(fn `UserConstructionScript`)